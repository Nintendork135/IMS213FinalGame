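; BP_Gate is a gate whose door opens once enough items have been collected.
; CollectItem increments a counter and, on reaching the maximum, fires OpenDoor through a DoOnce so it triggers only once.
; OpenDoor plays a timeline whose DoorTurn track drives a lerp on the Door component's relative yaw, swinging it open.
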(event Custom|Open%20Door
  (bind _door_turn (Timeline|Open%20Door%20Anim Play)
    (:Update
      (Transformation|SetRelativeRotation (Variables|Default|GetDoor) (Math|Rotator|MakeRotator 0.0 0.0 (Math|Float|Lerp -9e+01 1e+01 _door_turn)) false false))))

(event Custom|Collect%20Item
  (Math|Integer|IncrementInt (Variables|Default|GetcurrentItemsCollected)
    (:%20%20
      (if (>= (Variables|Default|GetcurrentItemsCollected) (Variables|Components|GetmaxItemsCollected))
        (Utilities|FlowControl|DoOnce false
          (:Completed
            (CallFunction|OpenDoor)))))))

(fn ConstructionScript)